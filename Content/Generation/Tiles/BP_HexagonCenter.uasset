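; BP_HexagonCenter is a generation tile for a hexagon center that randomizes its dressing of chairs and books on BeginPlay.
; It gives the Chairs and Books parent components random yaw, then runs each child through a random gate, destroying those that fail.
; Surviving books are child actors of BP_Book, raised in world Z by their HalfWidth.
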(event `self.ReceiveBeginPlay`
  (bind _returnvalue (`KismetMathLibrary.RandomFloatInRange` 0.0 360.0))
  (bind _books (`self.Books`))
  (`SceneComponent.K2_SetRelativeRotation` (`self.Chairs`) (`KismetMathLibrary.MakeRotator` 0.0 0.0 _returnvalue) false false)
  (`SceneComponent.K2_SetRelativeRotation` _books (`KismetMathLibrary.MakeRotator` 0.0 0.0 _returnvalue) false false)
  (bind (_arrayindex _arrayelement) (`/Engine/EditorBlueprintResources/StandardMacros.ReverseForEachLoop` (`SceneComponent.GetChildrenComponents` _books false))
    (:`LoopBody`
      (`/Game/Generation/ML_GenerationUtilities.RandomGate` 0.3
        (:`Pass`
          (bind _aschild_actor_component (cast `ChildActorComponent` _arrayelement))
          (bind _asbp_book (cast `/Game/Book/BP_Book` (`ChildActorComponent.ChildActor` _aschild_actor_component)))
          (`self.K2_AddActorWorldOffset` _asbp_book (`KismetMathLibrary.MakeVector` 0.0 0.0 (`Book.halfWidth` _asbp_book)) false false))
        (:`Fail`
          (`ActorComponent.K2_DestroyComponent` _arrayelement))))
    (:`Completed`
      (bind (_arrayindex_2 _arrayelement_2) (`/Engine/EditorBlueprintResources/StandardMacros.ReverseForEachLoop` (`SceneComponent.GetChildrenComponents` (`self.Chairs`) false))
        (:`LoopBody`
          (`/Game/Generation/ML_GenerationUtilities.RandomGate` 0.5
            (:`Fail`
              (`ActorComponent.K2_DestroyComponent` _arrayelement_2))))))))

(fn `UserConstructionScript`)