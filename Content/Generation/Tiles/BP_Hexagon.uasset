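; Hexagon level tile that populates its book rows and switches its lights as the player moves through it.
; The first player overlap of GenerateTrigger steps through child actors, randomly generating each BP_BookRow, with a short delay between rows while the player is distant to stagger the work.
; LightTrigger overlaps toggle all light components with on/off sounds.
; On BeginPlay, a CenterChance roll decides whether the Center component stays.
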(event `self.GenerateTrigger.OnComponentBeginOverlap`
  (params (OverlappedComponent :type "PrimitiveComponent Object Reference") (OtherActor :type "Actor Object Reference") (OtherComp :type "PrimitiveComponent Object Reference") (OtherBodyIndex :type Integer) (bFromSweep :type Boolean) (SweepResult :type "HitResult Structure (by ref)"))
  (bind _asbp_player (cast `/Game/Player/BP_Player` OtherActor))
  (`/Engine/EditorBlueprintResources/StandardMacros.DoOnce` false
    (:`Completed`
      (`self.GenerateBooks` _asbp_player))))

(event `GenerateBooks`
  (params (Player :type "Actor Object Reference"))
  (bind _childactors (`self.GetAllChildActors` true))
  (bind _currentindex (`self.CurrentIndex`))
  (bind _asbp_book_row (cast `/Game/Book/Row/BP_BookRow` (`|GetArrayItem` _childactors (`self.CurrentIndex`)) :!label _label)
    (:`then`
      (if (not (< (`KismetMathLibrary.Vector_Distance` (`self.K2_GetActorLocation` Player) (`SceneComponent.K2_GetComponentLocation` (`self.GenerateTrigger`))) 1000.0))
        (`KismetSystemLibrary.Delay` 0.2))
      (`/Game/Book/Row/BP_BookRow.GenerateBooksRandom` _asbp_book_row))
    (:`CastFailed`
      _))
  (`/Engine/EditorBlueprintResources/StandardMacros.IncrementInt` _currentindex
    (:`  `
      (if (< _currentindex (`KismetArrayLibrary.Array_Length` _childactors))
        (goto _label)))))

(event `SetLights`
  (params (On :type Boolean))
  (bind _returnvalue (`self.K2_GetActorLocation`))
  (for _array_element (`self.K2_GetComponentsByClass` "/Script/Engine.LightComponent")
    (`SceneComponent.SetVisibility` _array_element On false))
  (if On
    (`GameplayStatics.PlaySoundAtLocation` "/Game/Sound/SC_Lights_On.SC_Lights_On" _returnvalue (struct) 1.0 1.0 0.0 null null null)
    (else
      (`GameplayStatics.PlaySoundAtLocation` "/Game/Sound/SC_Lights_Off.SC_Lights_Off" _returnvalue (struct) 1.0 1.0 0.0 null null null))))

(event `self.LightTrigger.OnComponentBeginOverlap`
  (params (OverlappedComponent :type "PrimitiveComponent Object Reference") (OtherActor :type "Actor Object Reference") (OtherComp :type "PrimitiveComponent Object Reference") (OtherBodyIndex :type Integer) (bFromSweep :type Boolean) (SweepResult :type "HitResult Structure (by ref)"))
  (cast `/Game/Player/BP_Player` OtherActor)
  (`self.SetLights` true))

(event `self.LightTrigger.OnComponentEndOverlap`
  (params (OverlappedComponent :type "PrimitiveComponent Object Reference") (OtherActor :type "Actor Object Reference") (OtherComp :type "PrimitiveComponent Object Reference") (OtherBodyIndex :type Integer))
  (cast `/Game/Player/BP_Player` OtherActor)
  (`self.SetLights` false))

(event `self.ReceiveBeginPlay`
  (if (not (< (`KismetMathLibrary.RandomFloatInRange` 0.0 1.0) (`self.CenterChance`)))
    (`ActorComponent.K2_DestroyComponent` (`self.Center`))))

(fn `UserConstructionScript`)