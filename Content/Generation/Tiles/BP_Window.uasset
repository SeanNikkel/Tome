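; BP_Window is a tile window actor that toggles open and closed and can show a selected state.
; Toggle plays or reverses a timeline that pitches the whole actor's relative rotation up to -120 degrees.
; Timeline event tracks check playback direction to fire the matching open or close sound, if the caller requested sound.
; BeginPlay creates a dynamic material instance, whose Selected parameter SetSelected drives.
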(event `Toggle`
  (params (Sound :type Boolean :default true))
  (bind _returnvalue (`self.K2_GetActorLocation`))
  (set `self.PlaysSound` Sound)
  (bind _output_get (set `self.IsOpen` (not (`self.IsOpen`))))
  (if _output_get
    (bind (_direction _openamount) (`Timeline|OpenTimeline` :!label _label)
      (:`Update`
        (`self.K2_SetActorRelativeRotation` (`KismetMathLibrary.MakeRotator` 0.0 (* _openamount -120.0))))
      (:`CloseSound`
        (if (and (`|EnumEquality` _direction "Backward") (`self.PlaysSound`))
          (`GameplayStatics.PlaySoundAtLocation` "/Game/Sound/SC_WindowClose.SC_WindowClose" _returnvalue (struct) 1.0 1.0 0.0 null null null)))
      (:`OpenSound`
        (if (and (`|EnumEquality` _direction "Forward") (`self.PlaysSound`))
          (`GameplayStatics.PlaySoundAtLocation` "/Game/Sound/SC_WindowOpen.SC_WindowOpen" _returnvalue (struct) 1.0 1.0 0.0 null null null))))
    (else
      (goto _label :!via `Reverse`))))

(event `self.ReceiveBeginPlay`
  (bind _returnvalue (`PrimitiveComponent.CreateDynamicMaterialInstance` (`self.StaticMesh`) 0 "/Game/Generation/Tiles/M_Window.M_Window" "None"))
  (bind _output_get (set `self.WindowMaterial` _returnvalue))
  (`PrimitiveComponent.SetMaterial` (`self.StaticMesh`) 0 _output_get))

(fn `SetSelected`
  (params (Selected :type Boolean))
  (`MaterialInstanceDynamic.SetScalarParameterValue` (`self.WindowMaterial`) "Selected" (`KismetMathLibrary.Conv_BoolToDouble` Selected)))

(fn `UserConstructionScript`)