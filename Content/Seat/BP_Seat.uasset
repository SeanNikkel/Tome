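; BP_Seat is a seat actor that makes a BP_Player sit, attached at a raised offset, when the player overlaps its Box.
; GetExitPosition turns the local offsets from GetExitDirections into world orientation and picks the best dot-product match to the requested exit direction, returning that 2D position relative to the seat.
; GetExitDirections supplies a single forward offset here.
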(event `self.Box.OnComponentBeginOverlap`
  (params (OverlappedComponent :type "PrimitiveComponent Object Reference") (OtherActor :type "Actor Object Reference") (OtherComp :type "PrimitiveComponent Object Reference") (OtherBodyIndex :type Integer) (bFromSweep :type Boolean) (SweepResult :type "HitResult Structure (by ref)"))
  (bind _asbp_player (cast `/Game/Player/BP_Player` OtherActor))
  (`/Game/Player/BP_Player.Sit` _asbp_player self (0.0 0.0 80.0)))

(fn `GetExitDirections`
  (returns (Dirs :type "Array of Vector2D Structure"))
  (return (`|MakeArray` (100.0 0.0) :!type "Vector2D Structure")))

(fn `GetExitPosition`
  (params (ExitDir :type "Vector2D Structure"))
  (returns (WorldPos :type "Vector2D Structure"))
  (locals (ClosestVal :type "Float (double-precision)" :default -99999997952.0) (ClosestIndex :type Integer) (TransformedDirections :type "Array of Vector2D Structure"))
  (bind _dirs (`self.GetExitDirections`))
  (for _array_element _dirs
    (`KismetArrayLibrary.Array_Add` (`local.TransformedDirections`) (`KismetMathLibrary.Conv_VectorToVector2D` (`KismetMathLibrary.TransformDirection` (`self.GetTransform`) (`KismetMathLibrary.Conv_Vector2DToVector` _array_element)))))
  (for (_array_element_2 _array_index) (`local.TransformedDirections`)
    (bind _returnvalue (`KismetMathLibrary.DotProduct2D` (`KismetMathLibrary.Normal2D` _array_element_2) (`KismetMathLibrary.Normal2D` ExitDir)))
    (if (< (`local.ClosestVal`) _returnvalue)
      (set `local.ClosestVal` _returnvalue)
      (set `local.ClosestIndex` _array_index)))
  (return (+ (`|GetArrayItem` (`local.TransformedDirections`) (`local.ClosestIndex`)) (`KismetMathLibrary.Conv_VectorToVector2D` (`self.K2_GetActorLocation`)))))

(fn `UserConstructionScript`)