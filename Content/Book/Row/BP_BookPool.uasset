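; Actor pool that pre-spawns BP_Book actors for reuse in the generated library and cleans up distant ones.
; Tick adds one book per frame until PoolSize, attached to the pool and parked high in the sky.
; GetBook detaches and returns the first pooled book, or spawns one if empty.
; Tick also destroys unattached books beyond a squared radius from the player, derived from LibraryGenerator's RenderDistance and GridSize.
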(event `self.ReceiveBeginPlay`
  (bind _returnvalue (`GameplayStatics.GetActorOfClass` "/Script/LibraryOfBabel.LibraryGenerator"))
  (bind (_gridsize_x _gridsize_y _gridsize_z) (`KismetMathLibrary.BreakVector` (`LibraryGenerator.gridSize` _returnvalue)))
  (set `self.CleanRadiusSquared` (`KismetMathLibrary.Square` (- (`LibraryGenerator.renderDistance` _returnvalue) (`KismetMathLibrary.Sqrt` (* (`KismetMathLibrary.Square` (/ (`KismetMathLibrary.FMax` _gridsize_x _gridsize_y _gridsize_z) 2.0)) 3.0))))))

(event `self.ReceiveTick`
  (params (DeltaSeconds :type "Float (single-precision)"))
  (`|ExecutionSequence`
    (:`then_0`
      (if (< (`KismetArrayLibrary.Array_Length` (`self.Pool`)) (`self.PoolSize`))
        (`self.AddBook`)))
    (:`then_1`
      (bind _outactors (`GameplayStatics.GetAllActorsOfClass` "/Game/Book/BP_Book.BP_Book_C"))
      (for _array_element _outactors
        (bind _asbp_book (cast `/Game/Book/BP_Book` _array_element))
        (`/Engine/EditorBlueprintResources/StandardMacros.IsValid` (`self.GetAttachParentActor` _asbp_book)
          (:`Is Not Valid`
            (if (> (`KismetMathLibrary.Vector_DistanceSquared` (`self.K2_GetActorLocation` _asbp_book) (`self.K2_GetActorLocation` (`GameplayStatics.GetPlayerPawn` 0))) (`self.CleanRadiusSquared`))
              (`self.K2_DestroyActor` _asbp_book))))))))

(fn `AddBook`
  (bind _returnvalue (`|SpawnActorFromClass` "/Game/Book/BP_Book.BP_Book_C" (`KismetMathLibrary.MakeTransform` (0.0 0.0 0.0)) "Undefined" "OverrideRootScale" null null))
  (`self.K2_AttachToActor` _returnvalue self "None" "KeepRelative" "KeepRelative" "KeepRelative" true)
  (`KismetArrayLibrary.Array_Add` (`self.Pool`) _returnvalue)
  (`self.K2_SetActorLocation` _returnvalue (0.0 0.0 100000.0) false false))

(fn `GetBook`
  (returns (ReturnValue :type "Book Object Reference"))
  (locals (Result :type "Actor Object Reference"))
  (bind _pool (`self.Pool`))
  (if (== (`KismetArrayLibrary.Array_Length` _pool) 0)
    (bind _returnvalue (`|SpawnActorFromClass` "/Game/Book/BP_Book.BP_Book_C" (`KismetMathLibrary.MakeTransform` (0.0 0.0 0.0)) "Undefined" "OverrideRootScale" null null))
    (return _returnvalue)
    (else
      (bind _output_get (set `local.Result` (`|GetArrayItem` _pool)))
      (`KismetArrayLibrary.Array_Remove` (`self.Pool`))
      (`self.K2_DetachFromActor` _output_get "KeepRelative" "KeepRelative" "KeepRelative")
      (`self.K2_DetachFromActor` _output_get "KeepRelative" "KeepRelative" "KeepRelative")
      (bind _asbp_book (cast `/Game/Book/BP_Book` _output_get))
      (return _asbp_book))))

(fn `UserConstructionScript`)