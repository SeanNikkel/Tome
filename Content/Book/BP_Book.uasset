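; Book actor with randomized width, color and page count that opens, closes, turns pages and can become a physics object.
; Init seeds a stream for its look, with a rare one-page rainbow variant that cycles hue on Tick and shows a flying hint.
; Timelines swing the covers with sounds and move the book.
; SetPhysics hinges the simulated halves, then rebuilds root transform and opening angle from their pose when simulation ends.
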(event `self.ReceiveBeginPlay`
  (`self.Init`))

(event `ToggleOpen`
  (if (`|EnumEquality` (stale `OpenBook` _direction) "Forward")
    (`self.CloseBook`)
    (else
      (`self.OpenBook`))))

(event `OpenBook`
  (set `self.TargetAngle` (`self.HeldOpenAngle`))
  (`self.DisplayPage` (`self.currentPage`) null)
  (`|ExecutionSequence`
    (:`then_0`
      (if (`self.Rainbow`)
        (`TextRenderComponent.K2_SetText` (`self.FrontText`) "press f to fly")))
    (:`then_1`
      (set `self.StartAngle` (`self.CurrentAngle`) :!label _label)
      (bind (_direction _openamount) (`Timeline|Open` :!via `PlayFromStart`)
        (:`Update`
          (if (not (`self.PhysicsEnabled`))
            (bind _returnvalue (`KismetMathLibrary.RLerp` (`KismetMathLibrary.MakeRotator` (`self.StartAngle`)) (`KismetMathLibrary.MakeRotator` (`self.TargetAngle`)) _openamount))
            (set `self.CurrentAngle` (.roll _returnvalue))
            (`SceneComponent.K2_SetRelativeRotation` (`self.FrontMesh`) _returnvalue false false)
            (`SceneComponent.K2_SetRelativeRotation` (`self.BackMesh`) (`KismetMathLibrary.RLerp` (`KismetMathLibrary.MakeRotator` (* (`self.StartAngle`) -1.0)) (`KismetMathLibrary.MakeRotator` (* (`self.TargetAngle`) -1.0)) _openamount) false false)))
        (:`CloseSound`
          (if (== (`self.TargetAngle`) 0.0)
            (`GameplayStatics.PlaySoundAtLocation` "/Game/Sound/SC_BookClose.SC_BookClose" (`self.K2_GetActorLocation`) (struct) 1.0 1.0 0.0 null null null)))
        (:`OpenSound`
          (if (!= (`self.TargetAngle`) 0.0)
            (`GameplayStatics.PlaySoundAtLocation` "/Game/Sound/SC_BookOpen.SC_BookOpen" (`self.K2_GetActorLocation`) (struct) 1.0 1.0 0.0 null null null)))))))

(event `CloseBook`
  (set `self.TargetAngle` 0.0)
  (goto _label))

(event `self.ReceiveTick`
  (params (DeltaSeconds :type "Float (single-precision)"))
  (bind _returnvalue (`MaterialInstanceDynamic.K2_GetScalarParameterValue` (`self.BookMaterial`) "Hue"))
  (`MaterialInstanceDynamic.SetScalarParameterValue` (`self.BookMaterial`) "Hue" (`KismetMathLibrary.Fraction` (+ _returnvalue (/ DeltaSeconds 4.0)))))

(event `InterpTo`
  (params (Location :type "Vector Structure") (Rotation :type "Rotator Structure"))
  (bind _output_get (set `self.StartTransform` (`SceneComponent.GetRelativeTransform` (`self.SceneRoot`))))
  (bind (_direction _progress) (`Timeline|TransformInterp` :!via `PlayFromStart` :!label _label_2)
    (:`Update`
      (if (`self.PhysicsEnabled`)
        (goto _label_2 :!via `Stop`)
        (else
          (bind (_returnvalue_location _returnvalue_rotation) (`KismetMathLibrary.BreakTransform` (`KismetMathLibrary.TLerp` _output_get (`KismetMathLibrary.MakeTransform` Location Rotation) _progress)))
          (`SceneComponent.K2_SetRelativeLocationAndRotation` (`self.SceneRoot`) _returnvalue_location _returnvalue_rotation false false))))))

(event `self.EnablePhysics`
  (params (enable :type Boolean))
  (`self.SetPhysics` enable))

(event `self.PhysicsTeleport`
  (params (localPos :type "Vector Structure") (localRot :type "Rotator Structure"))
  (bind _returnvalue (`self.GetTransform` (`self.GetAttachParentActor`)))
  (bind _returnvalue_2 (`KismetMathLibrary.TransformLocation` _returnvalue localPos))
  (bind _returnvalue_3 (`KismetMathLibrary.TransformRotation` _returnvalue localRot))
  (`SceneComponent.K2_SetWorldLocationAndRotation` (`self.FrontMesh`) _returnvalue_2 _returnvalue_3 false true)
  (`SceneComponent.K2_SetWorldLocationAndRotation` (`self.BackMesh`) _returnvalue_2 _returnvalue_3 false true))

(fn `Init`
  (locals (Width :type "Float (double-precision)"))
  (bind (_widthscalarrange_x _widthscalarrange_y) (`KismetMathLibrary.BreakVector2D` (`self.WidthScalarRange`)))
  (bind (_pagecountrange_x _pagecountrange_y) (break `IntPoint` (`self.PageCountRange`)))
  (bind _returnvalue (`KismetMathLibrary.RandomFloatInRangeFromStream` 0.0 1.0 (`self.stream`)))
  (`self.SetSeed` (`KismetMathLibrary.RandomInteger` 2147483647))
  (bind _returnvalue_2 (`PrimitiveComponent.CreateDynamicMaterialInstance` (`self.BackMesh`) 0 "/Game/Book/M_Book.M_Book" "None"))
  (bind _output_get (set `self.BookMaterial` _returnvalue_2))
  (`PrimitiveComponent.SetMaterial` (`self.FrontMesh`) 0 _output_get)
  (set `local.Width` _returnvalue)
  (`self.SetWidth` (`KismetMathLibrary.Lerp` _widthscalarrange_x _widthscalarrange_y (`local.Width`)))
  (`/Game/Generation/ML_GenerationUtilities.RandomGate` 0.998
    (:`Pass`
      (`MaterialInstanceDynamic.SetScalarParameterValue` _output_get "Hue" _returnvalue)
      (`MaterialInstanceDynamic.SetScalarParameterValue` _output_get "Saturation" _returnvalue)
      (set `self.pageCount` (`KismetMathLibrary.Round` (`KismetMathLibrary.Lerp` (`KismetMathLibrary.Conv_IntToDouble` _pagecountrange_x) (`KismetMathLibrary.Conv_IntToDouble` _pagecountrange_y) (`local.Width`)))))
    (:`Fail`
      (`MaterialInstanceDynamic.SetScalarParameterValue` _output_get "Hue" 0.0)
      (`MaterialInstanceDynamic.SetScalarParameterValue` _output_get "Saturation" 1.0)
      (set `self.pageCount` 1)
      (set `self.Rainbow` true)
      (`self.SetActorTickEnabled` true)))
  (`self.GenerateOuterText`))

(fn `NextPage`
  (`self.DisplayPage` (+ (`self.currentPage`) 2) "/Game/Sound/SC_PageTurn.SC_PageTurn"))

(fn `PreviousPage`
  (`self.DisplayPage` (+ (`self.currentPage`) -2) "/Game/Sound/SC_PageTurn.SC_PageTurn"))

(fn `SetCollision`
  (params (Enabled :type Boolean))
  (bind _returnvalue (select `bool` Enabled :`false` "NoCollision" :`true` "QueryAndPhysics" :!type "ECollisionEnabled Enum"))
  (`PrimitiveComponent.SetCollisionEnabled` (`self.FrontMesh`) _returnvalue)
  (`PrimitiveComponent.SetCollisionEnabled` (`self.BackMesh`) _returnvalue))

(fn `SetPhysics`
  (params (Simulate :type Boolean))
  (locals (FrontNegative :type Boolean))
  (bind _returnvalue (`SceneComponent.K2_GetComponentRotation` (`self.FrontMesh`)))
  (bind _returnvalue_roll (`KismetMathLibrary.BreakRotator` (`KismetMathLibrary.InverseTransformRotation` (`SceneComponent.K2_GetComponentToWorld` (`self.BackMesh`)) _returnvalue)))
  (bind _output_get (set `self.PhysicsEnabled` Simulate))
  (`PrimitiveComponent.SetSimulatePhysics` (`self.FrontMesh`) _output_get)
  (`PrimitiveComponent.SetSimulatePhysics` (`self.BackMesh`) _output_get)
  (`self.SetCollision` _output_get)
  (if _output_get
    (`PhysicsConstraintComponent.SetConstrainedComponents` (`self.SpineHinge`) (`self.FrontMesh`) "None" (`self.BackMesh`) "None")
    (`self.DisplayPage` (`self.currentPage`) null)
    (else
      (`SceneComponent.K2_SetWorldLocation` (`self.SceneRoot`) (`SceneComponent.K2_GetComponentLocation` (`self.FrontMesh`)) false false)
      (`SceneComponent.K2_SetRelativeLocation` (`self.FrontMesh`) (0.0 0.0 0.0) false false)
      (`SceneComponent.K2_SetRelativeLocation` (`self.BackMesh`) (0.0 0.0 0.0) false false)
      (set `self.CurrentAngle` (`KismetMathLibrary.Abs` (/ _returnvalue_roll 2.0)))
      (`SceneComponent.K2_SetWorldRotation` (`self.SceneRoot`) (`KismetMathLibrary.MakeRotator` (- (.roll _returnvalue) (`self.CurrentAngle`)) (.pitch _returnvalue) (.yaw _returnvalue)) false false)
      (`SceneComponent.K2_SetRelativeRotation` (`self.FrontMesh`) (`KismetMathLibrary.MakeRotator` 0.0) false false)
      (`SceneComponent.K2_SetRelativeRotation` (`self.BackMesh`) (`KismetMathLibrary.MakeRotator` 0.0) false false)
      (`SceneComponent.K2_AttachToComponent` (`self.FrontMesh`) (`self.SceneRoot`) "None" "KeepRelative" "SnapToTarget" "KeepRelative" true)
      (`SceneComponent.K2_AttachToComponent` (`self.BackMesh`) (`self.SceneRoot`) "None" "KeepRelative" "SnapToTarget" "KeepRelative" true))))

(fn `SetSelected`
  (params (Selected :type Boolean))
  (`MaterialInstanceDynamic.SetScalarParameterValue` (`self.BookMaterial`) "Selected" (`KismetMathLibrary.Conv_BoolToDouble` Selected)))

(fn `SetWidth`
  (params (Scalar :type "Float (double-precision)"))
  (bind _frontmesh (`self.FrontMesh`))
  (bind (_returnvalue_x _returnvalue_y _returnvalue_z) (`KismetMathLibrary.BreakVector` (`SceneComponent.K2_GetComponentScale` (`self.BackMesh`))))
  (bind (_returnvalue_x_2 _returnvalue_y_2 _returnvalue_z_2) (`KismetMathLibrary.BreakVector` (`SceneComponent.K2_GetComponentScale` _frontmesh)))
  (bind _returnvalue (* Scalar _returnvalue_y_2))
  (set `self.halfWidth` (* _returnvalue (.y (`.BoxExtent` (`KismetMathLibrary.BreakBoxSphereBounds` (`StaticMesh.GetBounds` (`StaticMeshComponent.StaticMesh` _frontmesh))))) 2.0))
  (`SceneComponent.SetRelativeScale3D` (`self.FrontMesh`) (`KismetMathLibrary.MakeVector` _returnvalue_x_2 _returnvalue _returnvalue_z_2))
  (`SceneComponent.SetRelativeScale3D` (`self.BackMesh`) (`KismetMathLibrary.MakeVector` _returnvalue_x (* Scalar _returnvalue_y) _returnvalue_z))
  (`SceneComponent.SetWorldScale3D` (`self.FrontText`) (1.0 1.0 1.0))
  (`SceneComponent.SetWorldScale3D` (`self.FrontPageNum`) (1.0 1.0 1.0))
  (`SceneComponent.SetWorldScale3D` (`self.CoverText`) (1.0 1.0 1.0))
  (`SceneComponent.SetWorldScale3D` (`self.BackText`) (1.0 1.0 1.0))
  (`SceneComponent.SetWorldScale3D` (`self.BackPageNum`) (1.0 1.0 1.0))
  (`SceneComponent.SetWorldScale3D` (`self.FrontSpineText`) (1.0 1.0 1.0))
  (`SceneComponent.SetWorldScale3D` (`self.BackSpineText`) (1.0 1.0 1.0))
  (`self.UpdateSize`))

(fn `UpdateSize`
  (bind _frontmesh (`self.FrontMesh`))
  (bind (_returnvalue_origin _returnvalue_boxextent) (`KismetMathLibrary.BreakBoxSphereBounds` (`StaticMesh.GetBounds` (`StaticMeshComponent.StaticMesh` _frontmesh))))
  (bind (_returnvalue_x _returnvalue_y _returnvalue_z) (`KismetMathLibrary.BreakVector` (* _returnvalue_boxextent 2.0)))
  (set `self.Size` (* (`SceneComponent.K2_GetComponentScale` _frontmesh) (`KismetMathLibrary.MakeVector` _returnvalue_x (* _returnvalue_y 2.0) _returnvalue_z)))
  (return))

(fn `UserConstructionScript`)